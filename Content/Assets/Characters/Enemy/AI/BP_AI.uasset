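; Enemy AI character that senses, catches and can be stunned by the first-person player, reporting each state to its Blackboard.
; Pawn sensing flags the player as seen for a few seconds, while a Tick distance check flags a close-range catch.
; Overlapping the tagged flashlight (linterna) collider while it is on sets the stun flag, cleared when overlap ends.
; A Growl event plays randomized, time-limited audio, delayed after the first sound.
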(event OnSeePawn(PawnSensing)
  (params (Pawn :type Pawn%20Object%20Reference))
  (Utilities|Casting|CastToBP_FirstPersonCharacter Pawn)
  (AI|Components|Blackboard|SetValueasBool (AI|GetBlackboard (AI|GetAIController self)) (Utilities|Name|MakeLiteralName "hasSeenPlayer?") true)
  (Utilities|FlowControl|Delay 3.0)
  (AI|Components|Blackboard|SetValueasBool (AI|GetBlackboard (AI|GetAIController self)) (Utilities|Name|MakeLiteralName "hasSeenPlayer?") false))

(event OnComponentBeginOverlap(CapsuleComponent)
  (params (OverlappedComponent :type Primitive%20Component%20Object%20Reference) (OtherActor :type Actor%20Object%20Reference) (OtherComp :type Primitive%20Component%20Object%20Reference) (OtherBodyIndex :type Integer) (bFromSweep :type Boolean) (SweepResult :type Hit%20Result%20Structure%20%28by%20ref%29))
  (if (Variables|/Game/FirstPerson/Blueprints/BP_FirstPersonCharacter.BP_FirstPersonCharacter_C|GetlinternaActiva? (stale EventTick _asbp_first_person_character))
    (if (Components|ComponentHasTag OtherComp "LinternaCollider")
      (AI|Components|Blackboard|SetValueasBool (AI|GetBlackboard (AI|GetAIController self)) (Utilities|Name|MakeLiteralName "isStuned?") true)
      (Development|PrintString "true"))))

(event OnComponentEndOverlap(CapsuleComponent)
  (params (OverlappedComponent :type Primitive%20Component%20Object%20Reference) (OtherActor :type Actor%20Object%20Reference) (OtherComp :type Primitive%20Component%20Object%20Reference) (OtherBodyIndex :type Integer))
  (if (Components|ComponentHasTag OtherComp "LinternaCollider")
    (AI|Components|Blackboard|SetValueasBool (AI|GetBlackboard (AI|GetAIController self)) (Utilities|Name|MakeLiteralName "isStuned?") false)
    (Development|PrintString "falseeee")))

(event Custom|Growl
  (if (Variables|Default|GetmadeSound) :!label _label
    (Utilities|FlowControl|Delay 45.0))
  (if (< (Math|Random|RandomIntegerinRange 0 6) 4)
    (bind _returnvalue (AddComponent|AddAudioComponent false))
    (Audio|Components|Audio|StopDelayed _returnvalue 6.3)
    (Variables|Default|SetmadeSound true)
    (else
      (goto _label))))

(event EventTick
  (params (DeltaSeconds :type Float%20%28single-precision%29))
  (bind _asbp_first_person_character (Utilities|Casting|CastToBP_FirstPersonCharacter (Game|GetPlayerCharacter 0)))
  (if (< (Transformation|GetDistanceTo _asbp_first_person_character 0) 25.0)
    (AI|Components|Blackboard|SetValueasBool (AI|GetBlackboard (AI|GetAIController self)) (Utilities|Name|MakeLiteralName "caughtPlayer?") true)))

(fn ConstructionScript)