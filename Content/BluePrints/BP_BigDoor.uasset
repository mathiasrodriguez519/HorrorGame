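; BP_BigDoor is a door that the player swings open or closed with E, locked for as long as its Llave (key) reference is valid.
; Box1 enables input only while a component tagged VistaCollider overlaps it.
; Once Llave is invalid, each press alternates through a FlipFlop, adding an audio component and playing or reversing a timeline that lerps SMDoor's relative rotation between closed and open.
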(event OnComponentEndOverlap(Box1)
  (params (OverlappedComponent :type Primitive%20Component%20Object%20Reference) (OtherActor :type Actor%20Object%20Reference) (OtherComp :type Primitive%20Component%20Object%20Reference) (OtherBodyIndex :type Integer))
  (if (Components|ComponentHasTag OtherComp "VistaCollider")
    (Input|DisableInput (Game|GetPlayerController 0))))

(event OnComponentBeginOverlap(Box1)
  (params (OverlappedComponent :type Primitive%20Component%20Object%20Reference) (OtherActor :type Actor%20Object%20Reference) (OtherComp :type Primitive%20Component%20Object%20Reference) (OtherBodyIndex :type Integer) (bFromSweep :type Boolean) (SweepResult :type Hit%20Result%20Structure%20%28by%20ref%29))
  (if (Components|ComponentHasTag OtherComp "VistaCollider")
    (Input|EnableInput (Game|GetPlayerController 0))))

(event Input|KeyboardEvents|E
  (params (Key :type Key%20Structure))
  (:Pressed
    (Variables|Default|SetIsClose? (Utilities|IsValid (Variables|Default|GetLlave)))
    (if (not (Variables|Default|GetIsClose?))
      (Utilities|FlowControl|FlipFlop
        (:A
          (AddComponent|AddAudioComponent false)
          (bind _speed1 (Timeline|Open_close1 Play)
            (:Update
              (Transformation|SetRelativeRotation (Variables|Default|GetSM_Door) (Math|Rotator|Lerp(Rotator) (Variables|Default|GetClose1) (Variables|Default|GetOpen1) _speed1) false false))))
        (:B
          (AddComponent|AddAudioComponent false)
          (Timeline|Open_close1 Reverse))))))

(fn ConstructionScript)