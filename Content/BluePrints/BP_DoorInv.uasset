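; BP_DoorInv is a door that toggles open and closed with E, but only once the referenced key (Llave) is no longer valid.
; Overlapping Box1 with the first-person character enables input on the door, and leaving disables it.
; A FlipFlop plays or reverses the Open_close1 timeline, which lerps SMDoor's relative rotation between closed and open, with a sound for each direction.
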(event OnComponentEndOverlap(Box1)
  (params (OverlappedComponent :type Primitive%20Component%20Object%20Reference) (OtherActor :type Actor%20Object%20Reference) (OtherComp :type Primitive%20Component%20Object%20Reference) (OtherBodyIndex :type Integer))
  (Utilities|Casting|CastToBP_FirstPersonCharacter OtherActor)
  (Input|DisableInput (Game|GetPlayerController 0)))

(event OnComponentBeginOverlap(Box1)
  (params (OverlappedComponent :type Primitive%20Component%20Object%20Reference) (OtherActor :type Actor%20Object%20Reference) (OtherComp :type Primitive%20Component%20Object%20Reference) (OtherBodyIndex :type Integer) (bFromSweep :type Boolean) (SweepResult :type Hit%20Result%20Structure%20%28by%20ref%29))
  (Utilities|Casting|CastToBP_FirstPersonCharacter OtherActor)
  (Input|EnableInput (Game|GetPlayerController 0)))

(event Input|KeyboardEvents|E
  (params (Key :type Key%20Structure :default "None"))
  (:Pressed
    (Variables|Default|SetIsClose? (Utilities|IsValid (Variables|Default|GetLlave)))
    (if (not (Variables|Default|GetIsClose?))
      (Utilities|FlowControl|FlipFlop
        (:A
          (Audio|PlaySound2D "/Game/Assets/Sounds/door_opening.door_opening" 1.0 1.0 0.0 0 0)
          (bind _speed1 (Timeline|Open_close1 Play)
            (:Update
              (Transformation|SetRelativeRotation (Variables|Default|GetSM_Door) (Math|Rotator|Lerp(Rotator) (Variables|Default|GetClose1) (Variables|Default|GetOpen1) _speed1) false false))))
        (:B
          (Audio|PlaySound2D "/Game/Assets/Sounds/CloseDoor.CloseDoor" 1.0 1.0 0.0 0 0)
          (Timeline|Open_close1 Reverse))))))

(fn ConstructionScript)